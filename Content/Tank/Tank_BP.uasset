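; Player tank pawn Blueprint that wires input to the tank's movement, aiming and firing components.
; On BeginPlay it gives TankAiming the turret, barrel and projectile class, and TankMovement the two tracks.
; Move axes drive TankMovement, while Azimuth and Elevation rotate a camera gimbal and arm by a fixed step per input, unscaled by delta time.
; The Fire action calls TankAiming.Fire.
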(event `self.ReceiveBeginPlay`
  (`TankAimingComponent.Initialize` (`self.TankAiming`) (`self.TankTurret`) (`self.TankBarrel`) "/Game/Tank/Projectile_BP.Projectile_BP_C")
  (`TankMovementComponent.Initialize` (`self.TankMovement`) (`self.LeftTrack`) (`self.RightTrack`)))

(event `InputAxis|Azimuth`
  (params (AxisValue :type "Float (single-precision)"))
  ;[1 1 1] Aiming and Firing
  (`SceneComponent.K2_AddLocalRotation` (`self.AzimuthGimbal`) (`KismetMathLibrary.MakeRotator` 0.0 0.0 (* 5 AxisValue)) false false))

(event `InputAxis|Move Forward`
  (params (AxisValue :type "Float (single-precision)"))
  ;[1 1 1] Movement
  (`TankMovementComponent.MoveForward` (`self.TankMovement`) AxisValue))

(event `InputAxis|Move Right`
  (params (AxisValue :type "Float (single-precision)"))
  ;[1 1 1] Movement
  (`TankMovementComponent.MoveRight` (`self.TankMovement`) AxisValue))

(event `InputAxis|Elevation`
  (params (AxisValue :type "Float (single-precision)"))
  ;[1 1 1] Aiming and Firing
  (`SceneComponent.K2_AddLocalRotation` (`self.ElevationArm`) (`KismetMathLibrary.MakeRotator` 0.0 (* 5 AxisValue)) false false))

(event `InputAction|Fire`
  (params (Key :type "Key Structure"))
  ;[1 1 1] Aiming and Firing
  (:`Pressed`
    (`TankAimingComponent.Fire` (`self.TankAiming`))))

(fn `UserConstructionScript`)